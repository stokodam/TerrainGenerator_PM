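; NewGameMode is a game mode that puts up a start menu and launches hex map generation from its settings.
; The construction script, rather than BeginPlay, creates the MenuStart widget and adds it to the viewport.
; StartGenerating spawns BP_HexGenerator with the menu's noise, size, water, continent, biome and forest values, mapping SIzeX to Height and SizeY to Width, then removes the menu.
; The event graph handlers are empty.
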(event `self.ReceiveBeginPlay`)

(event `OnButtonClick`)

(fn `Start_generating`
  (bind _uimenu (`self.UIMenu`))
  (`|SpawnActorFromClass` "/Game/Generator/Blueprints/BP_HexGenerator.BP_HexGenerator_C" (`KismetMathLibrary.MakeTransform` (0.0 0.0 0.0)) "AlwaysSpawn" "MultiplyWithRoot" null (`/Game/Generator/Blueprints/MenuStart.TypeOdNoise` _uimenu) (`/Game/Generator/Blueprints/MenuStart.SIzeX` _uimenu) (`/Game/Generator/Blueprints/MenuStart.SizeY` _uimenu) (`/Game/Generator/Blueprints/MenuStart.WaterHeight` _uimenu) (`/Game/Generator/Blueprints/MenuStart.Scale` _uimenu) (`/Game/Generator/Blueprints/MenuStart.Continets` _uimenu) (`/Game/Generator/Blueprints/MenuStart.Desert` _uimenu) (`/Game/Generator/Blueprints/MenuStart.Snow` _uimenu) (`/Game/Generator/Blueprints/MenuStart.Tundra` _uimenu) (`/Game/Generator/Blueprints/MenuStart.ForestMin` _uimenu) (`/Game/Generator/Blueprints/MenuStart.ForestMax` _uimenu) null)
  (`Widget.RemoveFromParent` (`self.UIMenu`)))

(fn `UserConstructionScript`
  (bind _returnvalue (`|GenericCreateObject` "/Game/Generator/Blueprints/MenuStart.MenuStart_C"))
  (bind _output_get (set `self.UIMenu` _returnvalue))
  (`UserWidget.AddToViewport` _output_get 0))