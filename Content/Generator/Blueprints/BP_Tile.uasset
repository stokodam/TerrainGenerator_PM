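; BP_Tile is a generator tile that randomizes its own elevation in the construction script, becoming either water or land.
; A random roll picks the base water height about half the time, otherwise a separately rolled height clamped to a positive minimum.
; That height, scaled by strength plus an offset, shifts the static mesh vertically and also feeds the material's Elevation parameter.
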(event `self.ReceiveTick`
  (params (DeltaSeconds :type "Float (single-precision)")))

(fn `UserConstructionScript`
  (bind _returnvalue (`KismetMathLibrary.RandomFloatInRange` -1.0 1.0))
  (bind _staticmesh (`self.StaticMesh`))
  (if (<= _returnvalue 0.0)
    (set `self.Height` (`self.BaseWaterHeight`))
    (else
      (set `self.Height` (`KismetMathLibrary.FClamp` _returnvalue 0.1))))
  (`SceneComponent.K2_SetWorldLocation` _staticmesh (+ (`SceneComponent.K2_GetComponentLocation` _staticmesh) (`KismetMathLibrary.MakeVector` 0.0 0.0 (+ (* (`self.Height`) (`self.Strenght`)) (`self.Offset`)))) false false)
  (`MeshComponent.SetScalarParameterValueOnMaterials` (`self.StaticMesh`) "Elevation" (`self.Height`)))