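; BP_HexGenerator builds a hex-tile map with forests and a cube-built border at BeginPlay, then runs click-to-place scoring on it.
; Two FastNoise layers drive height and climate, with sine bias shaping climate and some continent modes.
; Tiles and woods are instanced meshes; per-instance custom data carries height, climate and biome thresholds.
; Clicking an unused tile adds a sprite and awards points, more beside earlier picks, updating the Points widget.
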(event `self.ReceiveBeginPlay`
  (bind _climatevalue (`self.ClimateValue`))
  (bind _scale (`self.Scale`))
  (bind _hexx (`self.HexX`))
  (bind _returnvalue (`StaticMesh.GetBoundingBox` (`self.TileMesh`)))
  (bind _returnvalue_2 (* (/ _hexx (`self.CubeX`)) (`self.Width`)))
  (bind _returnvalue_3 (`KismetMathLibrary.MakeVector` (* (/ (+ (`self.HexY`) (/ (`self.HexY`) 2.0)) (`self.CubeX`)) (/ (`self.Height`) 2)) 5.0 10.0))
  (bind _returnvalue_4 (`|GenericCreateObject` "/Script/FastNoiseGenerator.FastNoiseWrapper"))
  (bind _output_get (set `self.NoiseWrapper Lvl1` _returnvalue_4))
  (`FastNoiseWrapper.SetupFastNoise` _output_get (`self.Noise Type Lv1`) (`self.Seed Lv1`) (`self.Frequency Lv1`) (`self.Interp Lv1`) (`self.Fractaltype Lv1`) (`self.Octaves Lv1`) (`self.Lacunarity Lv1`) (`self.Gain Lv1`) (`self.Cellular Jitter Lv1`) (`self.Cellular Distance Function Lv1`) (`self.Cellular Return Type Lv1`))
  (bind _returnvalue_5 (`|GenericCreateObject` "/Script/FastNoiseGenerator.FastNoiseWrapper"))
  (bind _output_get_2 (set `self.NoiseWrapper Lvl2` _returnvalue_5))
  (`FastNoiseWrapper.SetupFastNoise` _output_get_2 (`self.Noise Type Lv2`) (`self.Seed Lv2`) (`self.Frequency Lv2`) (`self.Interp Lv2`) (`self.Fractaltype Lv2`) (`self.Octaves Lv2`) (`self.Lacunarity Lv2`) (`self.Gain Lv2`) (`self.Cellular Jitter Lv2`) (`self.Cellular Distance Function Lv2`) (`self.Cellular Return Type Lv2`))
  (`StaticMeshComponent.SetStaticMesh` (`self.Hex`) (`self.TileMesh`))
  (`StaticMeshComponent.SetStaticMesh` (`self.Woods`) (`self.WoodsMesh`))
  (set `self.Radius` (* (.x (`.Max` (break `Box` (`StaticMesh.GetBoundingBox` (`self.TileMesh`))))) (`self.Scale`)))
  (for _index (range 1 (+ (`self.Height`) 1))
    (for _index_2 (range 1 (+ (`self.Width`) 1))
      (bind (_x _y) (`self.CalculateOffset` _index_2 _index))
      (`self.NoiseGenerator` _index_2 _index)
      (bind _value (`self.GetNoiseValue` (`self.NoiseWrapper Lvl2`) (`KismetMathLibrary.Conv_IntToDouble` _index_2) (`KismetMathLibrary.Conv_IntToDouble` _index) _index (`self.Height`) 1))
      (set `self.ClimateValue` _value)
      (bind _returnvalue_6 (`InstancedStaticMeshComponent.AddInstance` (`self.Hex`) (`KismetMathLibrary.MakeTransform` (`KismetMathLibrary.MakeVector` _x _y (* (`self.HeightTile`) (`self.Scale Lv1`)))) false))
      (if (and (< _climatevalue (`self.ForestMaxValue`)) (> _climatevalue (`self.ForestMinValue`)) (> (`self.HeightTile`) (`self.Base Water Height`)))
        (`InstancedStaticMeshComponent.AddInstance` (`self.Woods`) (`KismetMathLibrary.MakeTransform` (`KismetMathLibrary.MakeVector` _x _y (+ (* (`self.HeightTile`) (`self.Scale Lv1`)) (.z (`.Max` (break `Box` (`StaticMesh.GetBoundingBox` (`self.TileMesh`))))))) (struct) (1.0 1.0 0.2)) false))
      (`InstancedStaticMeshComponent.SetCustomDataValue` (`self.Hex`) _returnvalue_6 0 (`self.HeightTile`) true)
      (`InstancedStaticMeshComponent.SetCustomDataValue` (`self.Hex`) _returnvalue_6 1 (`self.ClimateValue`) true)
      (`InstancedStaticMeshComponent.SetCustomDataValue` (`self.Hex`) _returnvalue_6 2 (`self.Base Water Height`) true)
      (`InstancedStaticMeshComponent.SetCustomDataValue` (`self.Hex`) _returnvalue_6 3 (`self.BaseDessertValue`) true)
      (`InstancedStaticMeshComponent.SetCustomDataValue` (`self.Hex`) _returnvalue_6 4 (`self.BaseSnowValue`) true)
      (`InstancedStaticMeshComponent.SetCustomDataValue` (`self.Hex`) _returnvalue_6 5 (`self.BaseTundraValue`) true))
    (`/Engine/EditorBlueprintResources/StandardMacros.FlipFlop`
      (:`A`
        (set `self.RowOffset` (* (`self.Radius`) -1.0)))
      (:`B`
        (set `self.RowOffset` 0.0))))
  (set `self.CubeX` (.x (`.Max` (break `Box` (`StaticMesh.GetBoundingBox` (`self.Cube`))))))
  (set `self.HexX` (* (.x (`.Max` (break `Box` _returnvalue))) _scale 2.0))
  (set `self.HexY` (* (.y (`.Max` (break `Box` _returnvalue))) _scale 2.0))
  (`|SpawnActorFromClass` "/Game/Generator/Blueprints/BP_Cube.BP_Cube_C" (`KismetMathLibrary.MakeTransform` (`KismetMathLibrary.MakeVector` (/ _hexx 2.0) -400.0) (struct) (`KismetMathLibrary.MakeVector` _returnvalue_2 5.0 10.0)) "AlwaysSpawn" "MultiplyWithRoot" null "/Game/StarterContent/Materials/M_Wood_Oak.M_Wood_Oak" null)
  (bind (_x_2 _y_2) (`self.CalculateOffset` 1 (`self.Height`)))
  (`|SpawnActorFromClass` "/Game/Generator/Blueprints/BP_Cube.BP_Cube_C" (`KismetMathLibrary.MakeTransform` (`KismetMathLibrary.MakeVector` (/ (`self.HexX`) 2.0) (+ _y_2 (/ (`self.HexY`) 4.0))) (struct) (`KismetMathLibrary.MakeVector` _returnvalue_2 5.0 10.0)) "AlwaysSpawn" "MultiplyWithRoot" null "/Game/StarterContent/Materials/M_Wood_Oak.M_Wood_Oak" null)
  (`|SpawnActorFromClass` "/Game/Generator/Blueprints/BP_Cube.BP_Cube_C" (`KismetMathLibrary.MakeTransform` (`KismetMathLibrary.MakeVector` (/ (`self.HexX`) 2.0) 100.0) (struct :`Yaw` 90.0) _returnvalue_3) "AlwaysSpawn" "MultiplyWithRoot" null "/Game/StarterContent/Materials/M_Wood_Oak.M_Wood_Oak" null)
  (bind (_x_3 _y_3) (`self.CalculateOffset` (`self.Width`) (`self.Height`)))
  (`|SpawnActorFromClass` "/Game/Generator/Blueprints/BP_Cube.BP_Cube_C" (`KismetMathLibrary.MakeTransform` (`KismetMathLibrary.MakeVector` _x_3 (+ _y_3 (/ (`self.HexY`) 4.0))) (struct :`Yaw` -90.0) _returnvalue_3) "AlwaysSpawn" "MultiplyWithRoot" null "/Game/StarterContent/Materials/M_Wood_Oak.M_Wood_Oak" null)
  (`|SpawnActorFromClass` "/Game/Generator/Blueprints/BP_Cube.BP_Cube_C" (`KismetMathLibrary.MakeTransform` (`KismetMathLibrary.MakeVector` (+ (/ (`self.HexX`) 2.0) -500.0) -400.0) (struct) (5.0 5.0 10.0)) "AlwaysSpawn" "MultiplyWithRoot" null "/Game/StarterContent/Materials/M_Metal_Chrome.M_Metal_Chrome" null)
  (bind (_x_4 _y_4) (`self.CalculateOffset` 1 (`self.Height`)))
  (`|SpawnActorFromClass` "/Game/Generator/Blueprints/BP_Cube.BP_Cube_C" (`KismetMathLibrary.MakeTransform` (`KismetMathLibrary.MakeVector` (+ (/ (`self.HexX`) 2.0) -500.01) (+ _y_4 (/ (`self.HexY`) 4.0)) 0.01) (struct) (5.0 5.0 10.0)) "AlwaysSpawn" "MultiplyWithRoot" null "/Game/StarterContent/Materials/M_Metal_Chrome.M_Metal_Chrome" null)
  (bind _x_5 (`self.CalculateOffset` (`self.Width`) (`self.Height`)))
  (`|SpawnActorFromClass` "/Game/Generator/Blueprints/BP_Cube.BP_Cube_C" (`KismetMathLibrary.MakeTransform` (`KismetMathLibrary.MakeVector` (+ _x_5 0.01) -400.01 0.01) (struct) (5.0 5.0 10.0)) "AlwaysSpawn" "MultiplyWithRoot" null "/Game/StarterContent/Materials/M_Metal_Chrome.M_Metal_Chrome" null)
  (bind (_x_6 _y_5) (`self.CalculateOffset` (`self.Width`) (`self.Height`)))
  (`|SpawnActorFromClass` "/Game/Generator/Blueprints/BP_Cube.BP_Cube_C" (`KismetMathLibrary.MakeTransform` (`KismetMathLibrary.MakeVector` (+ _x_6 0.01) (+ _y_5 (/ (`self.HexY`) 4.0) 0.01) 0.01) (struct) (5.0 5.0 10.0)) "AlwaysSpawn" "MultiplyWithRoot" null "/Game/StarterContent/Materials/M_Metal_Chrome.M_Metal_Chrome" null)
  (bind _returnvalue_7 (`|CreateWidget` "/Game/Generator/Blueprints/Points.Points_C"))
  (bind _output_get_3 (set `self.PointsUI` _returnvalue_7))
  (`UserWidget.AddToViewport` _output_get_3 0)
  (`/Game/Generator/Blueprints/Points.Change points` _output_get_3 "0"))

(event `self.Hex.OnReleased`
  (params (TouchedComponent :type "PrimitiveComponent Object Reference") (ButtonReleased :type "Key Structure"))
  (bind _prevlocation (`self.prevLocation`))
  (bind _location (.location (`InstancedStaticMeshComponent.GetInstanceTransform` (`self.Hex`) (`.HitItem` (`GameplayStatics.BreakHitResult` (`PlayerController.GetHitResultUnderCursorByChannel` (`GameplayStatics.GetPlayerController` 0) "TraceTypeQuery1" true))) true)))
  (if (not (`KismetArrayLibrary.Array_Contains` _prevlocation _location))
    (for _array_element _prevlocation
      (if (< (`KismetMathLibrary.Vector_Distance2D` _array_element _location) 174.0)
        (set `self.tempPoints` (+ (`self.tempPoints`) 2))))
    (if (< (`self.tempPoints`) 1)
      (set `self.points` (+ (`self.points`) 1))
      (else
        (set `self.points` (+ (`self.points`) (`self.tempPoints`)))))
    (set `self.tempPoints` 0)
    (`AddComponent|NODE_AddPaperSpriteComponent-1` :`RelativeTransform` (`KismetMathLibrary.MakeTransform` (+ _location (0.0 0.0 270.0)) (`KismetMathLibrary.MakeRotator` 90.0 (.pitch (.rotation (`InstancedStaticMeshComponent.GetInstanceTransform` (`self.Hex`) (`.HitItem` (`GameplayStatics.BreakHitResult` (`PlayerController.GetHitResultUnderCursorByChannel` (`GameplayStatics.GetPlayerController` 0) "TraceTypeQuery1" true))) true))) (.yaw (.rotation (`InstancedStaticMeshComponent.GetInstanceTransform` (`self.Hex`) (`.HitItem` (`GameplayStatics.BreakHitResult` (`PlayerController.GetHitResultUnderCursorByChannel` (`GameplayStatics.GetPlayerController` 0) "TraceTypeQuery1" true))) true)))) (`KismetMathLibrary.MakeVector` 0.5 0.5 0.5)))
    (`/Game/Generator/Blueprints/Points.Change points` (`self.PointsUI`) (`KismetTextLibrary.Conv_IntToText` (`self.points`)))
    (`KismetArrayLibrary.Array_Add` (`self.prevLocation`) _location)))

(fn `CalculateOffset`
  (params (Row :type Integer) (Heigh :type Integer))
  (returns (X :type "Float (double-precision)") (Y :type "Float (double-precision)"))
  (return (+ (* Row (`self.Radius`) 2.0) (* Row (`self.offset`)) (`self.RowOffset`)) (+ (* (/ (* (`self.Radius`) 2.0) (`KismetMathLibrary.Sqrt` 3.0)) 1.5 Heigh) (* Heigh (`self.offset`)))))

(fn `GetLorAValue`
  (params (NoiseType :type "FastNoiseWrapper Object Reference") (X :type "Float (double-precision)") (Y :type "Float (double-precision)"))
  (returns (Value :type "Float (double-precision)"))
  (locals (TempHeight :type "Float (double-precision)"))
  (bind _returnvalue (`FastNoiseWrapper.GetNoise2D` NoiseType X Y))
  (if (== 3 (`self.Continets`))
    (bind _result (`/Engine/EditorBlueprintResources/StandardMacros.NegateFloat` _returnvalue)
      (:`  `
        (set `local.TempHeight` (+ _result 0.25))))
    (else
      (set `local.TempHeight` _returnvalue)))
  (return (`local.TempHeight`)))

(fn `GetNoiseValue`
  (params (NewParam :type "FastNoiseWrapper Object Reference") (X :type "Float (double-precision)") (Y :type "Float (double-precision)") (RowID :type Integer) (WidthRow :type Integer) (PeriodSin :type Integer))
  (returns (Value :type "Float (double-precision)"))
  (return (+ (`FastNoiseWrapper.GetNoise2D` NewParam X Y) (- (* (`KismetMathLibrary.Abs` (`KismetMathLibrary.DegSin` (* (/ (`KismetMathLibrary.Conv_IntToDouble` RowID) (`KismetMathLibrary.Conv_IntToDouble` WidthRow)) (* (`KismetMathLibrary.Conv_IntToDouble` PeriodSin) 180.0)))) 2.0) 1.0))))

(fn `Height Generator`
  (returns (TileHeight :type "Float (double-precision)"))
  (bind _returnvalue (`KismetMathLibrary.RandomFloatInRange` -1.0 1.0))
  (if (<= _returnvalue 0.0)
    (set `self.HeightTile` (`self.Base Water Height`))
    (else
      (bind _output_get (set `self.HeightTile` (`KismetMathLibrary.FClamp` _returnvalue 0.1)))))
  (return (+ (* _output_get (`self.HeightStrenght`)) (`self.HeightOffset`))))

(fn `NoiseGenerator`
  (params (RowID :type Integer) (HeightID :type Integer))
  (bind _returnvalue (`KismetMathLibrary.Conv_IntToDouble` HeightID))
  (bind _returnvalue_2 (`KismetMathLibrary.Conv_IntToDouble` RowID))
  (switch `int` (`self.Continets`)
    (:`1`
      (bind _value (`self.GetNoiseValue` (`self.NoiseWrapper Lvl1`) _returnvalue_2 _returnvalue RowID (`self.Width`) (`self.Continets`) :!label _label))
      (if (<= _value (`self.Base Water Height`))
        (set `self.HeightTile` (`self.Base Water Height`))
        (else
          (set `self.HeightTile` _value))))
    (:`2`
      (goto _label))
    (:`3`
      (bind _value_2 (`self.GetLorAValue` (`self.NoiseWrapper Lvl1`) _returnvalue_2 _returnvalue :!label _label_2))
      (if (<= _value_2 (`self.Base Water Height`))
        (set `self.HeightTile` (`self.Base Water Height`))
        (else
          (set `self.HeightTile` _value_2))))
    (:`4`
      (goto _label_2)))
  (return))

(fn `UserConstructionScript`)